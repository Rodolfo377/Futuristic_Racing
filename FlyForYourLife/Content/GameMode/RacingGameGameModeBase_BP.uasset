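; Game mode Blueprint for a racing game that handles opening the gameplay level and creating the in-game UI.
; The LoadGameLevel event opens GuardRailLevel by name, while BeginPlay, Tick and the LoadLevel function are empty.
; LoadInGameWidget adds either a hover debug widget or the player's game UI to the viewport, depending on ShowHoverDebug.
; Leftover calls to LoadInGameWidget and StartGame are unwired and never run.
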(event `self.ReceiveBeginPlay`)

(event `self.ReceiveTick`
  (params (DeltaSeconds :type "Float (single-precision)")))

(event `LoadGameLevel`
  (`GameplayStatics.OpenLevel` "GuardRailLevel"))

(fn `LoadInGameWidget`
  (if (`self.ShowHoverDebug`)
    (bind _returnvalue (`|CreateWidget` "/Game/Widgets/DebugHovering.DebugHovering_C"))
    (bind _output_get (set `self.W_HoveringWidget` _returnvalue))
    (`UserWidget.AddToViewport` _output_get 0)
    (else
      (bind _returnvalue_2 (`|CreateWidget` "/Game/Widgets/W_GameUI.W_GameUI_C" (`GameplayStatics.GetPlayerController` 0)))
      (bind _output_get_2 (set `self.W_GameWidget` _returnvalue_2))
      (`UserWidget.AddToViewport` _output_get_2 0))))

(fn `LoadLevel`)

(fn `UserConstructionScript`)