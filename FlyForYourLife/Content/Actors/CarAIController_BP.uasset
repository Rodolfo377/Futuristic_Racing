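; AI controller for cars in the racing game that registers itself with the racing game mode on BeginPlay.
; Tick is empty, so the controller issues no movement in this graph.
; Disconnected waypoint-following logic remains: it prints and draws the game mode's current waypoint, calls MoveToLocation, and advances the index when already at the goal.
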(event `self.ReceiveBeginPlay`
  (bind _asracing_game_game_mode_base_bp (cast `/Game/GameMode/RacingGameGameModeBase_BP` (`GameplayStatics.GetGameMode`)))
  (`RacingGameGameModeBase.AddAIController` _asracing_game_game_mode_base_bp self))

(event `self.ReceiveTick`
  (params (DeltaSeconds :type "Float (single-precision)")))

(fn `UserConstructionScript`)