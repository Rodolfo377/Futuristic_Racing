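; Player hover-ship Blueprint for a racing game, caching its body and core meshes and the game mode on BeginPlay.
; Three stabilizer colliders snap-rotate the ship and swap material when touching Track-tagged actors.
; Input toggles a lowered center of mass or quits; ZTeleport overlaps reset position, and Wall hits apply an up-axis impulse, noted as not working.
; Hover PID and gravity debug displays exist but are disconnected.
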(event `self.ReceiveBeginPlay`
  (bind _returnvalue (`GameplayStatics.GetGameMode`))
  ;[1 1 1] Variables setup
  (set `self.ShipBody` (`self.ShipBodyMesh`))
  (set `self.ShipCore` (`self.ShipCoreMesh`))
  (`/Engine/EditorBlueprintResources/StandardMacros.IsValid` _returnvalue
    (:`Is Valid`
      (bind _asracing_game_game_mode_base_bp (cast `/Game/GameMode/RacingGameGameModeBase_BP` _returnvalue))
      (set `self.RacingGameMode` _asracing_game_game_mode_base_bp)
      (`WidgetBlueprintLibrary.SetInputMode_GameOnly` (`GameplayStatics.GetPlayerController` 0)))))

(event `InputAction|Escape`
  (params (Key :type "Key Structure"))
  ;[1 1 1] Quit Game by pressing ESC
  (:`Pressed`
    (`KismetSystemLibrary.QuitGame` null "Quit")))

(event `self.ReceiveActorBeginOverlap`
  (params (OtherActor :type "Actor Object Reference"))
  ;[1 1 1] "Kill Volume"
  (if (`self.ActorHasTag` OtherActor "ZTeleport")
    (`self.K2_SetActorLocation` (321.0 -2062.0 298.0) false true)))

(event `self.ReceiveHit`
  (params (MyComp :type "PrimitiveComponent Object Reference") (Other :type "Actor Object Reference") (OtherComp :type "PrimitiveComponent Object Reference") (bSelfMoved :type Boolean) (HitLocation :type "Vector Structure") (HitNormal :type "Vector Structure") (NormalImpulse :type "Vector Structure") (Hit :type "HitResult Structure (by ref)"))
  (bind _returnvalue (`self.GetActorUpVector`))
  ;[1 1 1] Impulse downwards on wall collisions so it keeps the ship on the track - Not working
  (if (`self.ActorHasTag` Other "Wall")
    (`PrimitiveComponent.AddImpulse` (`self.ShipCoreMesh`) (* _returnvalue (`KismetMathLibrary.Dot_VectorVector` NormalImpulse _returnvalue)) "None" false)))

(event `self.ReceiveTick`
  (params (DeltaSeconds :type "Float (single-precision)"))
  ;[1 1 1] Hover Debug information
)

(event `self.LeftStabilizer.OnComponentBeginOverlap`
  (params (OverlappedComponent :type "PrimitiveComponent Object Reference") (OtherActor :type "Actor Object Reference") (OtherComp :type "PrimitiveComponent Object Reference") (OtherBodyIndex :type Integer) (bFromSweep :type Boolean) (SweepResult :type "HitResult Structure (by ref)"))
  ;[1 1 1] left stabilizer functionality and visual feedback (dying red)
  (if (`self.ActorHasTag` OtherActor "Track")
    (`self.K2_AddActorLocalRotation` (struct :`Roll` 90.0))
    (`PrimitiveComponent.SetMaterial` (`self.LeftStabilizer`) 0 (`self.detectedStabilizer`))))

(event `self.LeftStabilizer.OnComponentEndOverlap`
  (params (OverlappedComponent :type "PrimitiveComponent Object Reference") (OtherActor :type "Actor Object Reference") (OtherComp :type "PrimitiveComponent Object Reference") (OtherBodyIndex :type Integer))
  ;[1 1 1] left stabilizer functionality and visual feedback (dying red)
  (if (`self.ActorHasTag` OtherActor "Track")
    (`KismetSystemLibrary.Delay` 1.0)
    (`PrimitiveComponent.SetMaterial` (`self.LeftStabilizer`) 0 (`self.normalStabilizer`))))

(event `self.RightStabilizer.OnComponentBeginOverlap`
  (params (OverlappedComponent :type "PrimitiveComponent Object Reference") (OtherActor :type "Actor Object Reference") (OtherComp :type "PrimitiveComponent Object Reference") (OtherBodyIndex :type Integer) (bFromSweep :type Boolean) (SweepResult :type "HitResult Structure (by ref)"))
  ;[1 1 1] right stabilizer functionality and visual feedback (dying red)
  (if (`self.ActorHasTag` OtherActor "Track")
    (`self.K2_AddActorLocalRotation` (struct :`Roll` -90.0))
    (`PrimitiveComponent.SetMaterial` (`self.RightStabilizer`) 0 (`self.detectedStabilizer`))))

(event `self.RightStabilizer.OnComponentEndOverlap`
  (params (OverlappedComponent :type "PrimitiveComponent Object Reference") (OtherActor :type "Actor Object Reference") (OtherComp :type "PrimitiveComponent Object Reference") (OtherBodyIndex :type Integer))
  ;[1 1 1] right stabilizer functionality and visual feedback (dying red)
  (if (`self.ActorHasTag` OtherActor "Track")
    (`KismetSystemLibrary.Delay` 1.0)
    (`PrimitiveComponent.SetMaterial` (`self.RightStabilizer`) 0 (`self.normalStabilizer`))))

(event `self.UpStabilizer.OnComponentBeginOverlap`
  (params (OverlappedComponent :type "PrimitiveComponent Object Reference") (OtherActor :type "Actor Object Reference") (OtherComp :type "PrimitiveComponent Object Reference") (OtherBodyIndex :type Integer) (bFromSweep :type Boolean) (SweepResult :type "HitResult Structure (by ref)"))
  ;[1 1 1] up stabilizer functionality and visual feedback (dying red)
  (if (`self.ActorHasTag` OtherActor "Track")
    (`self.K2_AddActorLocalRotation` (struct :`Roll` 180.0))
    (`PrimitiveComponent.SetMaterial` (`self.UpStabilizer`) 0 (`self.detectedStabilizer`))
    (`PrimitiveComponent.AddTorqueInDegrees` (`self.ShipCoreMesh`) (`self.GetActorForwardVector`) "None" false)))

(event `self.UpStabilizer.OnComponentEndOverlap`
  (params (OverlappedComponent :type "PrimitiveComponent Object Reference") (OtherActor :type "Actor Object Reference") (OtherComp :type "PrimitiveComponent Object Reference") (OtherBodyIndex :type Integer))
  ;[1 1 1] up stabilizer functionality and visual feedback (dying red)
  (if (`self.ActorHasTag` OtherActor "Track")
    (`KismetSystemLibrary.Delay` 1.0)
    (`PrimitiveComponent.SetMaterial` (`self.UpStabilizer`) 0 (`self.normalStabilizer`))))

(event `InputAction|ShiftCenterOfMass`
  (params (Key :type "Key Structure"))
  (:`Pressed`
    (`/Engine/EditorBlueprintResources/StandardMacros.FlipFlop`
      (:`A`
        (bind _output_get (set `self.Center Of Mass` (* (`self.GetActorUpVector`) (`self.DownOffset`))))
        (`PrimitiveComponent.SetCenterOfMass` (`self.ShipCoreMesh`) _output_get "None"))
      (:`B`
        (set `self.Center Of Mass` (0.0 0.0 0.0))
        (`PrimitiveComponent.SetCenterOfMass` (`self.ShipCoreMesh`) (0.0 0.0 0.0) "None")))))

(fn `NewFunction_0`)

(fn `UserConstructionScript`)