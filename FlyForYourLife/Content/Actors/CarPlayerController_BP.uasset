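; Player controller for a racing game that registers with the game mode and manages the race HUD and end screen.
; While the game loop is active, Tick has the game mode load the in-game widget if missing, then binds to the possessed car's lap and finish events.
; Completed laps refresh the HUD's lap times.
; Finishing swaps the HUD for the end-game widget with UI-only input and a visible cursor.
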(event `self.ReceiveBeginPlay`
  (bind _asracing_game_game_mode_base_bp (cast `/Game/GameMode/RacingGameGameModeBase_BP` (`GameplayStatics.GetGameMode`)))
  (`RacingGameGameModeBase.AddPlayerController` _asracing_game_game_mode_base_bp self))

(event `self.ReceiveTick`
  (params (DeltaSeconds :type "Float (single-precision)"))
  (bind _asracing_game_game_mode_base_bp (cast `/Game/GameMode/RacingGameGameModeBase_BP` (`GameplayStatics.GetGameMode`)))
  (if (`RacingGameGameModeBase.GameLoop` _asracing_game_game_mode_base_bp)
    (bind _output_get (set `self.In-Game Widget` (`/Game/GameMode/RacingGameGameModeBase_BP.W_GameWidget` _asracing_game_game_mode_base_bp)))
    (`/Engine/EditorBlueprintResources/StandardMacros.IsValid` _output_get
      (:`Is Not Valid`
        (bind _asracing_game_game_mode_base_bp_2 (cast `/Game/GameMode/RacingGameGameModeBase_BP` (`GameplayStatics.GetGameMode`)))
        (`/Game/GameMode/RacingGameGameModeBase_BP.LoadInGameWidget` _asracing_game_game_mode_base_bp_2)
        (cast `/Game/Actors/CustomCar_BP` (`self.K2_GetPawn`))
        (add `self.PlayerFinishedRace` (delegate `PlayerFinish`))
        (add `self.PlayerCompletedLap` (delegate `PlayerCompletedLap_Event_0`))))))

(event `PlayerCompletedLap_Event_0`
  (`/Game/Widgets/W_GameUI.UpdateLapTimes` (`self.In-Game Widget`)))

(event `PlayerFinish`
  (`Widget.RemoveFromParent` (`self.In-Game Widget`))
  (bind _returnvalue (`|CreateWidget` "/Game/Widgets/W_EndGame.W_EndGame_C"))
  (`UserWidget.AddToViewport` _returnvalue 0)
  (`WidgetBlueprintLibrary.SetInputMode_UIOnlyEx` self _returnvalue)
  (set `self.bShowMouseCursor` true))

(fn `UserConstructionScript`)