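; Hover vehicle prototype that drives a physics Cube with forces and torque; despite the name, it contains no spring or hover logic.
; Each Tick cancels sideways velocity with an acceleration force (also printed for debugging) and applies drag against forward speed, clamped to MaxSpeed.
; Accelerate and Steer axis events apply ForwardForce along forward and TurnTorque around up, without reading the axis value.
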(event `self.ReceiveTick`
  (params (DeltaSeconds :type "Float (single-precision)"))
  (bind _returnvalue (* (* (`self.GetActorRightVector`) (/ (`KismetMathLibrary.Dot_VectorVector` (`self.GetVelocity`) (`self.GetActorRightVector`)) (`GameplayStatics.GetWorldDeltaSeconds`))) -1.0))
  (`|ExecutionSequence`
    (:`then_2`
      ;[1 1 1] sideways friction
      (`KismetSystemLibrary.PrintString` (`KismetStringLibrary.Conv_VectorToString` _returnvalue))
      (`PrimitiveComponent.AddForce` (`self.Cube`) _returnvalue "None" true))
    (:`then_3`
      ;[1 1 1] Acceleration Friction
      (`PrimitiveComponent.AddForce` (`self.Cube`) (* (`self.GetActorForwardVector`) (* (* (`KismetMathLibrary.FClamp` (`KismetMathLibrary.Dot_VectorVector` (`self.GetVelocity`) (`self.GetActorForwardVector`)) 0.0 (`self.MaxSpeed`)) (`self.Drag`)) -1.0)) "None" true))))

(event `InputAxis|Accelerate`
  (params (AxisValue :type "Float (single-precision)"))
  ;[1 1 1] acceleration
  (`PrimitiveComponent.AddForce` (`self.Cube`) (* (`self.GetActorForwardVector`) (`self.ForwardForce`)) "None" true))

(event `InputAxis|Steer`
  (params (AxisValue :type "Float (single-precision)"))
  ;[1 1 1] steering
  (`PrimitiveComponent.AddTorqueInDegrees` (`self.Cube`) (* (`self.GetActorUpVector`) (`self.TurnTorque`)) "None" false))

(fn `UserConstructionScript`)