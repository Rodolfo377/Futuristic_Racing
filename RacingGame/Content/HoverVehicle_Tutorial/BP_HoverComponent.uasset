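; Hover point component for the BP_SpringHover vehicle, pushing its root body away from surfaces below as a spring-damper suspension.
; Each tick it traces along its negative up vector up to HoverDistance, with debug drawing.
; On a hit, it turns the compression and its rate of change into spring and damping force, applied along its up vector at the component's location, so offset placement also produces torque.
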(event `self.ReceiveBeginPlay`
  (bind _asbp_spring_hover (cast `/Game/HoverVehicle_Tutorial/BP_SpringHover` (`self.GetOwner`)))
  (set `self.ParentVehicle` _asbp_spring_hover))

(event `self.ReceiveTick`
  (params (DeltaSeconds :type "Float (single-precision)"))
  (bind _returnvalue (`self.K2_GetComponentLocation`))
  (`/Engine/EditorBlueprintResources/StandardMacros.IsValid` (`self.ParentVehicle`)
    (:`Is Valid`
      (bind _outhit (`KismetSystemLibrary.LineTraceSingle` :`Start` _returnvalue :`End` (- _returnvalue (* (`self.GetUpVector`) (`self.HoverDistance`))) :`TraceChannel` "TraceTypeQuery1" :`DrawDebugType` "ForOneFrame"))
      (if true
        (bind (_bblockinghit _binitialoverlap _time _distance) (`GameplayStatics.BreakHitResult` _outhit))
        (if _bblockinghit
          (bind _output_get (set `self.HoverDelta` (- (`self.HoverDistance`) _distance)))
          (bind _asprimitive_component (cast `PrimitiveComponent` (`Actor.RootComponent` (`self.ParentVehicle`))))
          (`PrimitiveComponent.AddForceAtLocation` _asprimitive_component (* (`self.GetUpVector`) (+ (* (/ (- _output_get (`self.PreviousHoverDelta`)) (`GameplayStatics.GetWorldDeltaSeconds`)) (`self.DampingCoefficient`)) (* _output_get (`self.SpringCoefficient`)))) (`self.K2_GetComponentLocation`) "None")
          (set `self.PreviousHoverDelta` (`self.HoverDelta`)))))))