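; CarAIController_BP is an AI controller that drives a car through the waypoint positions stored in RacingGameGameModeBase_BP.
; Every tick it reads the current waypoint from the game mode, prints it, draws a debug sphere there and reissues MoveToLocation toward it.
; An AlreadyAtGoal result advances the waypoint index, which has no wrap or bounds check here.
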(event `self.ReceiveTick`
  (params (DeltaSeconds :type "Float (single-precision)"))
  (bind _asracing_game_game_mode_base_bp (cast `/Game/GameMode/RacingGameGameModeBase_BP` (`GameplayStatics.GetGameMode`)))
  (bind _output (`|GetArrayItem` (`/Game/GameMode/RacingGameGameModeBase_BP.GM_WaypointPositions` _asracing_game_game_mode_base_bp) (`self.currentWaypoint`)))
  (`KismetSystemLibrary.PrintString` (`KismetStringLibrary.Conv_VectorToString` _output))
  (`KismetSystemLibrary.DrawDebugSphere` _output 100.0 12 (struct :`G` 0.142941 :`B` 1.0 :`A` 1.0))
  (bind _returnvalue (`self.MoveToLocation` _output -1.0 true true false true null))
  (if (`|EnumEquality` _returnvalue "AlreadyAtGoal")
    (set `self.currentWaypoint` (+ (`self.currentWaypoint`) 1))))

(fn `UserConstructionScript`)