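; Hover and custom-gravity component for CustomCar_BP, meant to float the ship body over track surfaces.
; Manager runs only Hovering, which traces toward a point missing the actor-location offset, stores hit height and normal, and pushes along that normal.
; Track alignment via cross-product axes and height-scaled gravity exist but are disconnected.
; Tick is disabled, nothing here calls Manager, and turning, counter-force and collision functions are empty stubs.
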(event `self.ReceiveBeginPlay`
  (bind _ascustom_car_bp (cast `/Game/Actors/CustomCar_BP` (`self.GetOwner`)))
  (set `self.OwnerActor` _ascustom_car_bp))

(fn `AlignShipWithTrack`
  (locals (CollisionObjects :type "Array of EObjectTypeQuery Enum"))
  (bind _tracknormal (`self.TrackNormal`))
  (bind _hitactor (`self.hitActor`))
  (bind _returnvalue (`Actor.GetActorForwardVector` (`self.OwnerActor`)))
  (bind _shipbody (`CustomCar.ShipBody` (`self.OwnerActor`)))
  (bind (_returnvalue_location _returnvalue_rotation) (`KismetMathLibrary.BreakTransform` (`SceneComponent.GetRelativeTransform` _shipbody)))
  (`/Engine/EditorBlueprintResources/StandardMacros.IsValid` _hitactor
    (:`Is Valid`
      (if (`Actor.ActorHasTag` _hitactor "Track")
        (`self.MyDebugDraw` _returnvalue (struct :`G` 1.0 :`B` 0.160949 :`A` 1.0))
        (bind _projectionontrack (`self.ProjectOnPlane` _returnvalue _tracknormal))
        (bind _returnvalue_2 (`KismetMathLibrary.Cross_VectorVector` _tracknormal _projectionontrack))
        (bind _returnvalue_3 (`KismetMathLibrary.Cross_VectorVector` _returnvalue_2 _tracknormal))
        (`self.MyDebugDraw` _returnvalue_3 (struct :`G` 0.958199 :`B` 0.970833 :`A` 1.0))
        (`self.MyDebugDraw` _returnvalue_2 (struct :`R` 0.024494 :`G` 0.008681 :`B` 1.0 :`A` 1.0))
        (bind _returnvalue_4 (`KismetMathLibrary.MakeRotationFromAxes` _returnvalue_3 _returnvalue_2 _tracknormal))
        (`SceneComponent.K2_SetWorldRotation` _shipbody _returnvalue_4 false false)
        (`SceneComponent.K2_SetRelativeRotation` _shipbody (`KismetMathLibrary.RLerp` _returnvalue_rotation _returnvalue_4 (`self.lerpAlpha`)) false false)))))

(fn `ApplyCustomGravity`
  (`PrimitiveComponent.AddForce` (`CustomCar.ShipBody` (`self.OwnerActor`)) (* (* (* (`self.TrackNormal`) -1.0) (`self.height`)) (`self.HoverGravity`)) "None" true))

(fn `CollisionImpulses`)

(fn `CounterForces`)

(fn `Hovering`
  (locals (HitObjects :type "Array of EObjectTypeQuery Enum") (forcePercent :type "Float (double-precision)") (totalHoverForce :type "Float (double-precision)"))
  (bind _returnvalue (`Actor.K2_GetActorLocation` (`self.OwnerActor`)))
  (bind _returnvalue_2 (* (* (`Actor.GetActorUpVector` (`self.OwnerActor`)) -1.0) (`self.HoveringDistance`)))
  (`self.MyDebugDraw` _returnvalue_2 (struct :`R` 0.989583 :`B` 0.320625 :`A` 1.0))
  (bind _outhit (`KismetSystemLibrary.LineTraceSingleForObjects` (`Actor.K2_GetActorLocation` (`self.OwnerActor`)) _returnvalue_2 (`local.HitObjects`)))
  (if (`GameplayStatics.BreakHitResult` _outhit)
    (`KismetSystemLibrary.PrintString` "BP_Custom gravity detected track!")
    (bind _output_get (set `self.height` (`.Distance` (`GameplayStatics.BreakHitResult` _outhit))))
    (set `self.TrackNormal` (`.Normal` (`GameplayStatics.BreakHitResult` _outhit)))
    (set `self.hitActor` (`.HitActor` (`GameplayStatics.BreakHitResult` _outhit)))
    (if (> _output_get (`self.HoveringDistance`))
      (bind _output_get_2 (set `local.forcePercent` 0.7))
      (set `local.totalHoverForce` (* _output_get_2 (`self.HoverForce`)))
      (else
        (bind _output_get_3 (set `local.forcePercent` 1.0))
        (set `local.totalHoverForce` (* _output_get_3 (`self.HoverForce`)))))
    (`PrimitiveComponent.AddForce` (`CustomCar.ShipBody` (`self.OwnerActor`)) (* (`self.TrackNormal`) (`local.totalHoverForce`)) "None" true)
    (`KismetSystemLibrary.DrawDebugLine` _returnvalue (+ _returnvalue (* (`self.TrackNormal`) 100.0)) (struct :`R` 0.951587 :`G` 1.0 :`B` 0.123273 :`A` 1.0) 0.0 3.0)))

(fn `Manager`
  (`|ExecutionSequence`
    (:`then_0`
      (`self.Hovering`))))

(fn `MyDebugDraw`
  (params (DrawVector :type "Vector Structure") (LineColor :type "LinearColor Structure"))
  (locals (MyLineColor :type "LinearColor Structure" :default (struct :`G` 0.076278 :`B` 1.0 :`A` 1.0)))
  (bind _returnvalue (`Actor.K2_GetActorLocation` (`self.OwnerActor`)))
  (set `local.MyLineColor` LineColor)
  (`KismetSystemLibrary.DrawDebugLine` _returnvalue (+ DrawVector _returnvalue) (`local.MyLineColor`) 0.0 8.0))

(fn `ProjectOnPlane`
  (params (ShipFwd :type "Vector Structure") (trackNormal :type "Vector Structure"))
  (returns (ProjectionOnTrack :type "Vector Structure"))
  (return (- ShipFwd trackNormal)))

(fn `Turning`)

(fn `UpdateRotatorAlpha`
  (bind _output_get (set `self.lerpAlpha` (+ (`self.lerpAlpha`) (* (`GameplayStatics.GetWorldDeltaSeconds`) 1.0))))
  (if (> _output_get 1.0)
    (set `self.lerpAlpha` 0.0)))